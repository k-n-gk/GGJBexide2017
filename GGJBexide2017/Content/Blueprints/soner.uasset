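; Sonar actor that emits a wave particle effect above its mesh every tick and flags detected zombies.
; Box hits or overlaps print the other actor's name and set HeriVisible on it if it is a zombie.
; A capsule hit from an Enemy-tagged actor starts a looping timer that drains HP until the sonar is destroyed, with nothing clearing the timer when contact ends.
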(event `self.ReceiveBeginPlay`)

(event `self.ReceiveTick`
  (params (DeltaSeconds :type "Float (single-precision)"))
  (`GameplayStatics.SpawnEmitterAtLocation` "/Game/ParticleSystem/wave.wave" (`KismetMathLibrary.MakeVector` (.x (`SceneComponent.K2_GetComponentLocation` (`self.StaticMesh`))) (.y (`SceneComponent.K2_GetComponentLocation` (`self.StaticMesh`))) (+ (.z (`SceneComponent.K2_GetComponentLocation` (`self.StaticMesh`))) 200.0))))

(event `self.Capsule.OnComponentHit`
  (params (HitComponent :type "PrimitiveComponent Object Reference") (OtherActor :type "Actor Object Reference") (OtherComp :type "PrimitiveComponent Object Reference") (NormalImpulse :type "Vector Structure") (Hit :type "HitResult Structure (by ref)"))
  (if (`KismetArrayLibrary.Array_Contains` (`Actor.Tags` OtherActor) "Enemy")
    (`KismetSystemLibrary.K2_SetTimerDelegate` (delegate `カスタムイベント_0`) 0.1 true)))

(event `カスタムイベント_0`
  (bind _output_get (set `self.HP` (- (`self.HP`) 1.0)))
  (if (<= _output_get 0.0)
    (`self.K2_DestroyActor`)))

(event `self.Box.OnComponentHit`
  (params (HitComponent :type "PrimitiveComponent Object Reference") (OtherActor :type "Actor Object Reference") (OtherComp :type "PrimitiveComponent Object Reference") (NormalImpulse :type "Vector Structure") (Hit :type "HitResult Structure (by ref)"))
  (`KismetSystemLibrary.PrintString` (`KismetSystemLibrary.GetDisplayName` (stale `self.Box.OnComponentBeginOverlap` OtherActor)) :!label _label)
  (bind _aszombie (cast `/Game/enemyBP/zombie` (stale `self.Box.OnComponentBeginOverlap` OtherActor)))
  (set `/Game/enemyBP/zombie.HeriVisible` true _aszombie))

(event `self.Box.OnComponentBeginOverlap`
  (params (OverlappedComponent :type "PrimitiveComponent Object Reference") (OtherActor :type "Actor Object Reference") (OtherComp :type "PrimitiveComponent Object Reference") (OtherBodyIndex :type Integer) (bFromSweep :type Boolean) (SweepResult :type "HitResult Structure (by ref)"))
  (goto _label))

(fn `UserConstructionScript`)