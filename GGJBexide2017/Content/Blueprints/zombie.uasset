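; Zombie enemy that seeks the nearest target from its ZombieManager, switches to attack in close range and loses health to Bullet-tagged hits.
; A Move/Attack/Crawl/Die state machine runs on Tick, with ChangeState setting each looping or one-shot animation and play rate.
; Low health forces crawling, and zero health disables capsule collision and sinks the body, with a timer check for destruction.
; HeriVisible toggles a StaticMesh material each frame.
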(event `self.ReceiveBeginPlay`
  (`self.ChangeState` "NewEnumerator0" true)
  (set `self.leftHealth` (`self.defaultHealth`)))

(event `self.ReceiveTick`
  (params (DeltaSeconds :type "Float (single-precision)"))
  (bind _returnvalue (`self.K2_GetActorLocation`))
  (bind _staticmesh (`self.StaticMesh`))
  (`|ExecutionSequence`
    (:`then_0`
      (if (<= (`self.leftHealth`) 0)
        (`self.ChangeState` "NewEnumerator3")
        (if (`self.HeriVisible`) :!label _label
          (`PrimitiveComponent.SetMaterial` _staticmesh 0 "/Game/particle/wa2_Mat2.wa2_Mat2")
          (else
            (`PrimitiveComponent.SetMaterial` _staticmesh 0 "/Game/StarterContent/Materials/M_Glass.M_Glass")))
        (if (`|EnumEquality` (`self.state`) "NewEnumerator0")
          (`|ExecutionSequence` :!label _label_2
            (:`then_0`
              (bind (_nearestposition _targetactor) (`/Game/FirstPersonBP/Blueprints/ZombieManager.GetNearestTargetPosition` (`self.zombieManager`) _returnvalue))
              (set `self.targetPosition` (`KismetMathLibrary.MakeVector` (.x _nearestposition) (.y _nearestposition) (.z _returnvalue)))
              (set `self.targetActor` _targetactor))
            (:`then_1`
              (`NavigationSystem.SimpleMoveToLocation` (`self.GetController`) (`self.targetPosition`)))
            (:`then_2`
              (bind _returnvalue_2 (`self.CheckTargetInAttackArea` 100.0))
              (if _returnvalue_2
                (`self.ChangeState` "NewEnumerator1"))))
          (elif (`|EnumEquality` (`self.state`) "NewEnumerator1")
            (if (== (`self.targetActor`) null)
              (`self.ChangeState` "NewEnumerator0"))
            (elif (`|EnumEquality` (`self.state`) "NewEnumerator2")
              (goto _label_2)
              (elif (`|EnumEquality` (`self.state`) "NewEnumerator3")
                (`self.K2_AddActorWorldOffset` (0.0 0.0 -1.0) false true)
                (if (>= (+ (`self.DiedSec`) DeltaSeconds) 5.0)
                  (`self.K2_DestroyActor`))))))))
    (:`then_1`
      (if (< (`self.leftHealth`) (`self.dyingHealthBorder`))
        (`self.ChangeState` "NewEnumerator2")
        (goto _label)))
    (:`then_2`
      (goto _label))))

(event `self.ReceiveHit`
  (params (MyComp :type "PrimitiveComponent Object Reference") (Other :type "Actor Object Reference") (OtherComp :type "PrimitiveComponent Object Reference") (bSelfMoved :type Boolean) (HitLocation :type "Vector Structure") (HitNormal :type "Vector Structure") (NormalImpulse :type "Vector Structure") (Hit :type "HitResult Structure (by ref)"))
  (if (`KismetArrayLibrary.Array_Contains` (`Actor.Tags` Other) "Bullet")
    (`/Engine/EditorBlueprintResources/StandardMacros.DecrementInt` (`self.leftHealth`))))

(fn `ChangeState`
  (params (newState :type "/Game/enemyBP/EZombieState Enum") (forceChange :type Boolean))
  (locals (_newState :type "/Game/enemyBP/EZombieState Enum"))
  (if (or (`|EnumInequality` newState (`self.state`)) forceChange)
    (set `local._newState` newState)
    (`SkeletalMeshComponent.PlayAnimation` (`self.Mesh`) (select `/Game/enemyBP/EZombieState` (`local._newState`) :`NewEnumerator0` "/Game/Zombie_01/manequinretarget/Zombie_Walk_F_1_Loop_IP.Zombie_Walk_F_1_Loop_IP" :`NewEnumerator1` "/Game/Zombie_01/manequinretarget/Zombie_Atk_Loop_1_IP.Zombie_Atk_Loop_1_IP" :`NewEnumerator2` "/Game/Zombie_01/manequinretarget/Zombie_Crawl_1_Loop_IP.Zombie_Crawl_1_Loop_IP" :`NewEnumerator3` "/Game/Zombie_01/manequinretarget/Zombie_Death_Back_Mid_1_IP.Zombie_Death_Back_Mid_1_IP" :!type "AnimationAsset Object Reference") (select `/Game/enemyBP/EZombieState` (`local._newState`) :`NewEnumerator0` true :`NewEnumerator1` true :`NewEnumerator2` true))
    (`SkeletalMeshComponent.SetPlayRate` (`self.Mesh`) (select `/Game/enemyBP/EZombieState` (`local._newState`) :`NewEnumerator0` 5.0 :`NewEnumerator1` 3.0 :`NewEnumerator2` 3.0 :`NewEnumerator3` 1.0 :!type "Float (single-precision)"))
    (bind _output_get (set `self.state` (`local._newState`)))
    (if (`|EnumEquality` _output_get "NewEnumerator3")
      (`PrimitiveComponent.SetCollisionEnabled` (`self.CapsuleComponent`) "NoCollision"))))

(fn `CheckTargetInAttackArea`
  (params (border :type "Float (double-precision)"))
  (returns (ReturnValue :type Boolean))
  (return (< (`KismetMathLibrary.VSizeSquared` (- (`self.K2_GetActorLocation`) (`self.targetPosition`))) (`KismetMathLibrary.Square` border))))

(fn `IsNearCanditatePosition`
  (params (CanditatePosition :type "Vector Structure"))
  (returns (ReturnValue :type Boolean))
  (bind _returnvalue (`self.K2_GetActorLocation`))
  (return (< (`KismetMathLibrary.VSizeSquared` (- CanditatePosition _returnvalue)) (`KismetMathLibrary.VSizeSquared` (- _returnvalue (`self.targetPosition`))))))

(fn `SetZombieManager`
  (params (zombieManager :type "/Game/FirstPersonBP/Blueprints/ZombieManager Object Reference"))
  (set `self.zombieManager` zombieManager))

(fn `UserConstructionScript`)