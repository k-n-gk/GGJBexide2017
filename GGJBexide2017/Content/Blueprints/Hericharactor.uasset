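; Hericharactor is an actor Blueprint that fires at the point under the mouse cursor on left click.
; The click traces the Visibility channel, stores the hit location as Aimlocation in Mygamestate and moves the Sphere component there.
; It then spawns a Bulletactor and Bullet particle effect at the StaticMesh's location, plus a Soner actor raised above the cursor's hit point.
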(event `Key|LeftMouseButton`
  (params (Key :type "Key Structure" :default "AnyKey"))
  (bind _returnvalue (`SceneComponent.K2_GetComponentLocation` (`self.StaticMesh`)))
  (bind (_bblockinghit _binitialoverlap _time _location) (`GameplayStatics.BreakHitResult` (`PlayerController.GetHitResultUnderCursorByChannel` (`GameplayStatics.GetPlayerController` 0) "TraceTypeQuery1" true)))
  (:`Pressed`
    (bind _output_get (set `/Game/Blueprints/Mygamestate.aimlocation` _location (cast `/Game/Blueprints/Mygamestate` (`GameplayStatics.GetGameState`) :!pure true)))
    (`SceneComponent.K2_SetWorldLocation` (`self.Sphere`) _output_get false false)
    (`|SpawnActorFromClass` "/Game/Blueprints/bulletactor.bulletactor_C" (`KismetMathLibrary.Conv_VectorToTransform` _returnvalue) "Undefined" "OverrideRootScale")
    (`GameplayStatics.SpawnEmitterAtLocation` "/Game/ParticleSystem/bullet.bullet" _returnvalue (struct))
    (`|SpawnActorFromClass` "/Game/Blueprints/soner.soner_C" (`KismetMathLibrary.Conv_VectorToTransform` (`KismetMathLibrary.MakeVector` (.x _location) (.y _location) (+ (.z _location) 200.0))) "Undefined" "OverrideRootScale")))

(fn `UserConstructionScript`)